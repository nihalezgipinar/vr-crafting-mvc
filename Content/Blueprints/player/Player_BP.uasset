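; VR player Blueprint that lets the user grab and release objects with left and right motion controllers.
; BeginPlay sets a local-floor tracking origin and adds the Enhanced Input mapping context.
; Pressing grab runs a zero-length sphere trace at that controller and grips the hit component, or else its actor, if it implements VRGripInterface.
; Releasing grab drops that controller's gripped objects through the same interface.
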(event Custom|AttemptToGripFromTrace
  (params (CallingController :type Grip%20Motion%20Controller%20Component%20Object%20Reference))
  (bind (_hitresult _hit) (CallFunction|TracefromController CallingController))
  (if _hit
    (CallFunction|AttemptoGrip _hitresult CallingController)))

(event Input|EnhancedActionEvents|EnhancedInputActionGrabLeft_IA
  (params (ActionValue :type Boolean) (ElapsedSeconds :type Float%20%28double-precision%29) (TriggeredSeconds :type Float%20%28double-precision%29) (InputAction :type Input%20Action%20Object%20Reference :default "/Game/Blueprints/player/PlayerInput/GrabLeft_IA.GrabLeft_IA"))
  (bind _gripmotioncontroller_l (Variables|Default|GetGripMotionController_L))
  (:Started
    (CallFunction|AttempttoGripfromTrace _gripmotioncontroller_l))
  (:Completed
    (CallFunction|DropAllGrips _gripmotioncontroller_l)))

(event Input|EnhancedActionEvents|EnhancedInputActionGrabRight_IA
  (params (ActionValue :type Boolean) (ElapsedSeconds :type Float%20%28double-precision%29) (TriggeredSeconds :type Float%20%28double-precision%29) (InputAction :type Input%20Action%20Object%20Reference :default "/Game/Blueprints/player/PlayerInput/GrabRight_IA.GrabRight_IA"))
  (bind _gripmotioncontroller_r (Variables|Default|GetGripMotionController_R))
  (:Started
    (CallFunction|AttempttoGripfromTrace _gripmotioncontroller_r))
  (:Completed
    (CallFunction|DropAllGrips _gripmotioncontroller_r)))

(event EventBeginPlay
  (Class|HeadMountedDisplayFunctionLibrary|SetTrackingOrigin "LocalFloor")
  (bind _asplayer_controller (Utilities|Casting|CastToPlayerController (Pawn|GetController)))
  (Input|AddMappingContext (PlayerController|LocalPlayerSubsystems|GetEnhancedInputLocalPlayerSubsystem _asplayer_controller) "/Game/Blueprints/player/PlayerInput/PlayerInput_IMC.PlayerInput_IMC" 0 "(bIgnoreAllPressedKeysUntilRelease=True,bForceImmediately=False,bNotifyUserSettings=False)"))

(event Collision|EventActorBeginOverlap
  (params (OtherActor :type Actor%20Object%20Reference)))

(event EventTick
  (params (DeltaSeconds :type Float%20%28single-precision%29)))

(fn ConstructionScript)

(fn DropAllGrips
  (params (CallingController :type Grip%20Motion%20Controller%20Component%20Object%20Reference))
  (if (Class|GripMotionControllerComponent|HasGrippedObjects CallingController)
    (bind _grippedobjectsarray (Class|GripMotionControllerComponent|GetGrippedObjects CallingController))
    (for _array_element _grippedobjectsarray
      (if (Utilities|DoesObjectImplementInterface _array_element "/Script/VRExpansionPlugin.VRGripInterface")
        (Class|GripMotionControllerComponent|DropObjectbyInterface CallingController _array_element 0 "0, 0, 0" "0, 0, 0")))))

(fn AttemptoGrip
  (params (HitResult :type Hit%20Result%20Structure) (CallingController :type Grip%20Motion%20Controller%20Component%20Object%20Reference))
  (bind (_bblockinghit _binitialoverlap _time _distance _location _impactpoint _normal _impactnormal _physmat _hitactor _hitcomponent) (Collision|BreakHitResult HitResult))
  ;[0.15 0.15 0.15 0.5] Component
  (if (Utilities|DoesObjectImplementInterface _hitcomponent "/Script/VRExpansionPlugin.VRGripInterface")
    (Class|GripMotionControllerComponent|GripObjectbyInterface CallingController _hitcomponent (Transformation|GetWorldTransform _hitcomponent) false "None" "None" false)
    (else
      ;[0.15 0.15 0.15 0.5] Actor
      (if (Utilities|DoesObjectImplementInterface _hitactor "/Script/VRExpansionPlugin.VRGripInterface")
        (Class|GripMotionControllerComponent|GripObjectbyInterface CallingController _hitactor (Transformation|GetActorTransform _hitactor) false "None" "None" false)))))

(fn TracefromController
  (params (CallingController :type Grip%20Motion%20Controller%20Component%20Object%20Reference))
  (bind _returnvalue (Transformation|GetWorldLocation CallingController))
  (bind (_outhit _returnvalue_2) (Collision|SphereTraceByChannel _returnvalue _returnvalue 7.0 "TraceTypeQuery1" false 0 "None"))
  (return _outhit _returnvalue_2))