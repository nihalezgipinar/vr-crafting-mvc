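; Display board actor that shows crafting results on a DisplayBoardUI widget held by its widget component.
; UpdateDisplayBoard receives whether a recipe was found, plus its name, produced value and image, and passes them to UpdateUI.
; A failed lookup substitutes a "Recipe not Found!" message and red exclamation icon.
; UpdateUI hides the instructions, sets the results title and reveals the produced, name and icon fields.
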(event Custom|UpdateDisplayBoard
  (params (found :type Boolean) (RecipeName :type String) (Produced :type String) (Result%20Image :type Texture%202D%20Object%20Reference))
  (bind _asdisplay_board_ui (Utilities|Casting|CastToDisplayBoardUI (UserInterface|GetWidget (Variables|Default|GetDisplayBoardUI))))
  (if found
    (CallFunction|UpdateUI _asdisplay_board_ui RecipeName Produced Result%20Image)
    (else
      (CallFunction|UpdateUI _asdisplay_board_ui "Recipe not Found!" "" "/Game/UI/UIBoardsAndImages/Exclamation_Red.Exclamation_Red"))))

(event EventBeginPlay)

(event Collision|EventActorBeginOverlap
  (params (OtherActor :type Actor%20Object%20Reference)))

(event EventTick
  (params (DeltaSeconds :type Float%20%28single-precision%29)))

(fn ConstructionScript)

(fn UpdateUI
  (params (DisplayBoardUIRef :type Display%20Board%20UI%20Object%20Reference) (RecipeName :type String) (Produced :type String) (ResultImage :type Texture%202D%20Object%20Reference))
  (bind _imageicon (Variables|/Game/UI/DisplayBoardUI.DisplayBoardUI_C|GetImageIcon DisplayBoardUIRef))
  (bind _producedtext (Variables|/Game/UI/DisplayBoardUI.DisplayBoardUI_C|GetProducedText DisplayBoardUIRef))
  (Variables|/Script/UMG.Widget|SetVisibility (Variables|/Game/UI/DisplayBoardUI.DisplayBoardUI_C|GetInstructionsText DisplayBoardUIRef) "Hidden")
  (Variables|/Script/UMG.TextBlock|SetText (Variables|/Game/UI/DisplayBoardUI.DisplayBoardUI_C|GetTitleText DisplayBoardUIRef) "CRAFTING RESULTS")
  (Variables|/Script/UMG.Widget|SetVisibility _producedtext "Visible")
  (Variables|/Script/UMG.TextBlock|SetText _producedtext (Utilities|Text|ToText(String) Produced))
  (Variables|/Script/UMG.Widget|SetVisibility (Variables|/Game/UI/DisplayBoardUI.DisplayBoardUI_C|GetRecipeName DisplayBoardUIRef) "Visible")
  (Variables|/Script/UMG.TextBlock|SetText (Variables|/Game/UI/DisplayBoardUI.DisplayBoardUI_C|GetRecipeName DisplayBoardUIRef) (Utilities|Text|ToText(String) RecipeName))
  (Variables|/Script/UMG.Widget|SetVisibility _imageicon "Visible")
  (Class|Image|SetBrush _imageicon (Utilities|Struct|MakeSlateBrush "(SpecifiedColor=(R=1.000000,G=1.000000,B=1.000000,A=1.000000),ColorUseRule=UseColor_Specified)" "Image" "NoTile" "NoMirror" "(X=32.000000,Y=32.000000)" "(Left=0.000000,Top=0.000000,Right=0.000000,Bottom=0.000000)" ResultImage "(CornerRadii=(X=0.000000,Y=0.000000,Z=0.000000,W=0.000000),Color=(SpecifiedColor=(R=0.000000,G=0.000000,B=0.000000,A=0.000000),ColorUseRule=UseColor_Specified),Width=0.000000,RoundingType=HalfHeightRadius,bUseBrushTransparency=False)")))