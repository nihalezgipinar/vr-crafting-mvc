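; Hopper controller that pairs two incoming ingredients and shows the resulting recipe on a display board.
; Hopperinfo alternately stores each ingredient's class in the first and second slot, evaluating the pair on every second call.
; Identical ingredients update the board with no recipe data.
; Differing pairs are matched in either order against every recipe data table row, passing the found flag, title, description and image to the board.
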(event Custom|Hopperinfo
  (params (Ingredient :type Ingredient%20Object%20Reference))
  (bind _returnvalue (Utilities|GetClass Ingredient))
  ;[0.15 0.15 0.15 0.5] First and second ingredient
  (if (== (Variables|Default|Geti) 0)
    (Utilities|Array|SetArrayElem (Variables|Default|GetIngredients) 0 _returnvalue)
    (Math|Integer|IncrementInt (Variables|Default|Geti))
    (else
      (Utilities|Array|SetArrayElem (Variables|Default|GetIngredients) 1 _returnvalue)
      (Variables|Default|Seti 0)
      (Variables|Default|Setfound false)
      ;[0.15 0.15 0.15 0.5] Are both ingredients the same?
      (if (== (Utilities|Array|Get(acopy) (Variables|Default|GetIngredients)) (Utilities|Array|Get(acopy) (Variables|Default|GetIngredients) 1))
        (Default|UpdateDisplayBoard (Variables|Default|GetDisplayBoard) false)
        (else
          (bind _outrownames (DataTable|GetDataTableRowNames "/Game/RecipeDataTable.RecipeDataTable"))
          (for _array_element _outrownames
            (bind _returnvalue_2 (Utilities|GetDataTableRow "/Game/RecipeDataTable.RecipeDataTable" _array_element)
              (:then
                (if (and (or (== (Utilities|Array|Get(acopy) (Variables|Default|GetIngredients)) (.FirstIngredirent (Utilities|Struct|BreakRecipe _returnvalue_2))) (== (Utilities|Array|Get(acopy) (Variables|Default|GetIngredients)) (.SecondIngredient (Utilities|Struct|BreakRecipe _returnvalue_2)))) (or (== (Utilities|Array|Get(acopy) (Variables|Default|GetIngredients) 1) (.FirstIngredirent (Utilities|Struct|BreakRecipe _returnvalue_2))) (== (Utilities|Array|Get(acopy) (Variables|Default|GetIngredients) 1) (.SecondIngredient (Utilities|Struct|BreakRecipe _returnvalue_2)))))
                  (Variables|Default|Setfound true)
                  (Variables|Default|SetResult%20Title (.ResultTitle (Utilities|Struct|BreakRecipe _returnvalue_2)))
                  (Variables|Default|Setresult%20Image (.ResultImage (Utilities|Struct|BreakRecipe _returnvalue_2)))
                  (Variables|Default|SetProduced (.ResultDescription (Utilities|Struct|BreakRecipe _returnvalue_2)))))))
          (Default|UpdateDisplayBoard (Variables|Default|GetDisplayBoard) (Variables|Default|Getfound) (Variables|Default|GetResult%20Title) (Variables|Default|GetProduced) (Variables|Default|Getresult%20Image)))))))

(event EventBeginPlay)

(event Collision|EventActorBeginOverlap
  (params (OtherActor :type Actor%20Object%20Reference)))

(event EventTick
  (params (DeltaSeconds :type Float%20%28single-precision%29)))

(fn ConstructionScript)